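; BP_CrunchDummy is a dummy actor, filed under Player, that shows its health on a widget gauge.
; Its HealthUpdated event casts the widget component's user widget to ValueGauge, stores it as HealthBar and, if valid, sets it to the current and maximum health.
; The default BeginPlay, overlap and Tick events are disabled, and the construction script only calls its parent.
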(event EventBeginPlay
  (|CallParentFunction) ; This node is disabled and will not be called.\nDrag off pins to build functionality.
)

(event Collision|EventActorBeginOverlap
  (params (OtherActor :type Actor%20Object%20Reference))
  (|CallParentFunction OtherActor) ; This node is disabled and will not be called.\nDrag off pins to build functionality.
)

(event EventTick
  (params (DeltaSeconds :type Float%20%28single-precision%29))
  (|CallParentFunction DeltaSeconds) ; This node is disabled and will not be called.\nDrag off pins to build functionality.
)

(event EventHealthUpdated
  (params (Health :type Float%20%28single-precision%29) (healthDelta :type Float%20%28single-precision%29) (maxHealth :type Float%20%28single-precision%29))
  (bind _asvalue_gauge (Utilities|Casting|CastToValueGauge (UserInterface|GetUserWidgetObject (Variables|Default|GetWidget))))
  (bind _output_get (Variables|Default|SetHealthBar _asvalue_gauge))
  (Utilities|IsValid _output_get
    (:Is%20Valid
      (Default|SetValue _output_get Health maxHealth))))

(fn ConstructionScript
  (|CallParentFunction))